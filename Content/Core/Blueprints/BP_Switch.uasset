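; BP_Switch is an interactable wall or lever switch that toggles power on a Target, gated by a Breaker's power state.
; NarrativeInteractable triggers the toggle and shows open/close action text from the switch state.
; With power, fast looping timers step the mesh's roll to its end position, then send SetPowerMessage to the Target.
; Without power, the mesh briefly flicks and snaps back after a short delay.
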(event OnInteracted(NarrativeInteractable)
  (params (Interactor :type Pawn%20Object%20Reference) (InteractionComp :type Narrative%20Interaction%20Component%20Object%20Reference))
  (bind _on_ (Class|BPIElectricObject|GetPowerState(Message) (Variables|Default|GetBreaker)))
  (if _on_
    (if (Variables|Default|GetSwitchPowerOn?)
      (Variables|Default|SetSwitchPowerOn? false)
      (CallFunction|SetTextAction)
      (bind _returnvalue (Utilities|Time|SetTimerbyFunctionName 0 "SwitchOff" 0.001 true))
      (Variables|Default|SetSwitchOff_TimerHandle _returnvalue)
      (else
        (Variables|Default|SetSwitchPowerOn? true)
        (CallFunction|SetTextAction)
        (bind _returnvalue_2 (Utilities|Time|SetTimerbyFunctionName 0 "SwitchOn" 0.001 true))
        (Variables|Default|SetSwitchOn_TimerHandle _returnvalue_2)))
    (else
      (Transformation|SetRelativeRotation (Variables|Default|GetStaticMesh) (Math|Rotator|MakeRotator (Variables|Default|GetTarget%20Rotation_Open) 0.0 0.0) false false)
      (Utilities|FlowControl|Delay 0.2)
      (Transformation|SetRelativeRotation (Variables|Default|GetStaticMesh) (Math|Rotator|MakeRotator (Variables|Default|GetTarget%20Rotation_Close) 0.0 0.0) false false))))

(event Custom|Init
  (bind _on_ (Class|BPIElectricObject|GetPowerState(Message) (Variables|Default|GetBreaker)))
  (if _on_
    (Class|BPIElectricObject|SetPower(Message) (Variables|Default|GetTarget))
    (CallFunction|SetTextAction)
    (CallFunction|CEInteracted)))

(event Custom|CE_Interacted
  (bind _on_ (Class|BPIElectricObject|GetPowerState(Message) (Variables|Default|GetBreaker)))
  (if _on_
    (if (Variables|Default|GetSwitchPowerOn?)
      (Variables|Default|SetSwitchPowerOn? false)
      (CallFunction|SetTextAction)
      (bind _returnvalue (Utilities|Time|SetTimerbyFunctionName 0 "SwitchOff" 0.001 true))
      (Variables|Default|SetSwitchOff_TimerHandle _returnvalue)
      (else
        (Variables|Default|SetSwitchPowerOn? true)
        (CallFunction|SetTextAction)
        (bind _returnvalue_2 (Utilities|Time|SetTimerbyFunctionName 0 "SwitchOn" 0.001 true))
        (Variables|Default|SetSwitchOn_TimerHandle _returnvalue_2)))
    (else
      (Transformation|SetRelativeRotation (Variables|Default|GetStaticMesh) (Math|Rotator|MakeRotator (Variables|Default|GetTarget%20Rotation_Open) 0.0 0.0) false false)
      (Utilities|FlowControl|Delay 0.2)
      (Transformation|SetRelativeRotation (Variables|Default|GetStaticMesh) (Math|Rotator|MakeRotator (Variables|Default|GetTarget%20Rotation_Close) 0.0 0.0) false false))))

(event Custom|SwitchOn
  (Transformation|SetRelativeRotation (Variables|Default|GetStaticMesh) (Math|Rotator|MakeRotator (Math|Interpolation|FInterptoConstant (Variables|Default|GetCurrentRotation) (Variables|Default|GetTarget%20Rotation_Open) (Utilities|Time|GetWorldDeltaSeconds) (Variables|Default|GetActivateSpeed)) 0.0 0.0) false false)
  (bind _output_get (Variables|Default|SetCurrentRotation (select (Variables|Default|GetSwitchPowerOn?) (- (Variables|Default|GetCurrentRotation) 1.0) (+ (Variables|Default|GetCurrentRotation) 1.0))))
  (if (== _output_get (select (Variables|Default|GetSwitchPowerOn?) (Variables|Default|GetTarget%20Rotation_Open) (Variables|Default|GetTarget%20Rotation_Close)))
    (Utilities|Time|ClearandInvalidateTimerbyHandle (Variables|Default|GetSwitchOn_TimerHandle))
    (Class|BPIElectricObject|SetPower(Message) (Variables|Default|GetTarget))))

(event Custom|SwitchOff
  (Transformation|SetRelativeRotation (Variables|Default|GetStaticMesh) (Math|Rotator|MakeRotator (Math|Interpolation|FInterptoConstant (Variables|Default|GetCurrentRotation) (Variables|Default|GetTarget%20Rotation_Close) (Utilities|Time|GetWorldDeltaSeconds) (Variables|Default|GetActivateSpeed)) 0.0 0.0) false false)
  (bind _output_get (Variables|Default|SetCurrentRotation (select (Variables|Default|GetSwitchPowerOn?) (- (Variables|Default|GetCurrentRotation) 1.0) (+ (Variables|Default|GetCurrentRotation) 1.0))))
  (if (== _output_get (select (Variables|Default|GetSwitchPowerOn?) (Variables|Default|GetTarget%20Rotation_Open) (Variables|Default|GetTarget%20Rotation_Close)))
    (Utilities|Time|ClearandInvalidateTimerbyHandle (Variables|Default|GetSwitchOff_TimerHandle))
    (Class|BPIElectricObject|SetPower(Message) (Variables|Default|GetTarget))))

(event EventResetState
  (if (Variables|Default|GetSwitchPowerOn?)
    (Class|BPIElectricObject|SetPower(Message) (Variables|Default|GetTarget))))

(event EventSetPower
  (bind _on_ (Class|BPIElectricObject|GetPowerState(Message) (Variables|Default|GetBreaker)))
  (if _on_
    (if (Variables|Default|GetSwitchPowerOn?)
      (Variables|Default|SetSwitchPowerOn? true)
      (else
        (Variables|Default|SetSwitchPowerOn? false)))
    (elif (Variables|Default|GetSwitchPowerOn?)
      _)))

(fn ConstructionScript)

(fn SetTextAction
  (Class|NarrativeInteractableComponent|SetInteractableActionText (Variables|Default|GetNarrativeInteractable) (select (Variables|Default|GetSwitchPowerOn?) (Variables|Default|GetCloseText) (Variables|Default|GetOpenText))))

(fn SetTargetRotation
  (if (not (Variables|Default|GetSwitchPowerOn?))
    (Variables|Default|SetTargetRotation (Variables|Default|GetTarget%20Rotation_Open))
    (Transformation|SetRelativeRotation (Variables|Default|GetStaticMesh) (Math|Rotator|MakeRotator (Variables|Default|GetTarget%20Rotation_Open) 0.0 0.0) false false)
    (else
      (Variables|Default|SetTargetRotation (Variables|Default|GetTarget%20Rotation_Close))
      (Transformation|SetRelativeRotation (Variables|Default|GetStaticMesh) (Math|Rotator|MakeRotator (Variables|Default|GetTarget%20Rotation_Close) 0.0 0.0) false false))))

(fn GetPowerState
  (return (Variables|Default|GetSwitchPowerOn?)))