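; Interactable breaker switch that flips a mesh lever and turns a linked TargetBreaker's power on or off.
; A Narrative interaction toggles PowerOn and starts a fast looping timer that rotates the mesh's roll toward the on or off angle.
; CurrentRotation steps one degree per tick; on exactly matching the target, the timer clears, TargetBreaker receives the power message and the interaction text updates.
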(event OnInteracted(NarrativeInteractable)
  (params (Interactor :type Pawn%20Object%20Reference) (InteractionComp :type Narrative%20Interaction%20Component%20Object%20Reference))
  (if (Variables|Default|GetPowerOn?)
    (Variables|Default|SetPowerOn? false)
    (bind _returnvalue (Utilities|Time|SetTimerbyFunctionName 0 "SwitchBreakOff" 0.001 true))
    (Variables|Default|SetBreakerOff_TimerHandle _returnvalue)
    (else
      (Variables|Default|SetPowerOn? true)
      (bind _returnvalue_2 (Utilities|Time|SetTimerbyFunctionName 0 "SwitchBreakOn" 0.001 true))
      (Variables|Default|SetBreakerOn_TimerHandle _returnvalue_2))))

(event Custom|SwitchBreakOff
  (Transformation|SetRelativeRotation (Variables|Default|GetStaticMesh) (Math|Rotator|MakeRotator (Math|Interpolation|FInterptoConstant (Variables|Default|GetCurrentRotation) (Variables|Default|GetTarget%20Rotation_PowerOff) (Utilities|Time|GetWorldDeltaSeconds) (Variables|Default|GetActivateSpeed)) 0.0 0.0) false false)
  (bind _output_get (Variables|Default|SetCurrentRotation (select (Variables|Default|GetPowerOn?) (- (Variables|Default|GetCurrentRotation) 1.0) (+ (Variables|Default|GetCurrentRotation) 1.0))))
  (if (== _output_get (select (Variables|Default|GetPowerOn?) (Variables|Default|GetTarget%20Rotation_PowerOn) (Variables|Default|GetTarget%20Rotation_PowerOff)))
    (Utilities|Time|ClearandInvalidateTimerbyHandle (Variables|Default|GetBreakerOff_TimerHandle))
    (CallFunction|SetTextAction)
    (Class|BPIElectricObject|SetPoweron(Message) (Variables|Default|GetTargetBreaker) false)))

(event Custom|SwitchBreakOn
  (Transformation|SetRelativeRotation (Variables|Default|GetStaticMesh) (Math|Rotator|MakeRotator (Math|Interpolation|FInterptoConstant (Variables|Default|GetCurrentRotation) (Variables|Default|GetTarget%20Rotation_PowerOn) (Utilities|Time|GetWorldDeltaSeconds) (Variables|Default|GetActivateSpeed)) 0.0 0.0) false false)
  (bind _output_get (Variables|Default|SetCurrentRotation (select (Variables|Default|GetPowerOn?) (- (Variables|Default|GetCurrentRotation) 1.0) (+ (Variables|Default|GetCurrentRotation) 1.0))))
  (if (== _output_get (select (Variables|Default|GetPowerOn?) (Variables|Default|GetTarget%20Rotation_PowerOn) (Variables|Default|GetTarget%20Rotation_PowerOff)))
    (Utilities|Time|ClearandInvalidateTimerbyHandle (Variables|Default|GetBreakerOn_TimerHandle))
    (Class|BPIElectricObject|SetPoweron(Message) (Variables|Default|GetTargetBreaker) true)
    (CallFunction|SetTextAction)))

(event EventBeginPlay
  (Transformation|SetRelativeRotation (Variables|Default|GetStaticMesh) (Math|Rotator|MakeRotator (select (Variables|Default|GetPowerOn?) (Variables|Default|GetTarget%20Rotation_PowerOn) (Variables|Default|GetTarget%20Rotation_PowerOff)) 0.0 0.0) false false)
  (Variables|Default|SetCurrentRotation (select (Variables|Default|GetPowerOn?) (Variables|Default|GetTarget%20Rotation_PowerOn) (Variables|Default|GetTarget%20Rotation_PowerOff)))
  (CallFunction|SetTextAction))

(fn ConstructionScript)

(fn SetTextAction
  (Class|NarrativeInteractableComponent|SetInteractableActionText (Variables|Default|GetNarrativeInteractable) (select (Variables|Default|GetPowerOn?) (Variables|Default|GetPowerOff_Text) (Variables|Default|GetPowerON_Text))))

(fn GetPowerState
  (return (Variables|Default|GetPowerOn?)))