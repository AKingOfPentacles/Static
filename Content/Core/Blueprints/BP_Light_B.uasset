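; BP_Light_B is a light prop that is lit only when both its PowerBox and its Switch report power.
; BeginPlay creates a dynamic material for the bulb mesh to control its emissive intensity.
; SetPower queries both power states, then sets bulb glow and the visibility of every light in Lights to match.
; GetPowerState always returns false, and the node filling Lights with the two point lights is disconnected.
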(event EventBeginPlay
  (bind _returnvalue (Rendering|Material|CreateDynamicMaterialInstance (Variables|Default|GetSM_Prop_Light_Bulb_01) 0 "/Game/PolygonHorrorMansion/Materials/Alts/M_PolygonHorrorMansion_Mat_01_A.M_PolygonHorrorMansion_Mat_01_A" "None" :!class /Script/Engine.PrimitiveComponent))
  (Variables|Default|SetMID_IntensityEmissive _returnvalue))

(event EventSetPower
  (bind _on_ (Class|BPIElectricObject|GetPowerState(Message) (Variables|Default|GetPowerBox)))
  (if _on_
    (bind _on__2 (Class|BPIElectricObject|GetPowerState(Message) (Variables|Default|GetSwitch)))
    (Rendering|Material|SetScalarParameterValue (Variables|Default|GetMID_IntensityEmissive) "Intensity" (select _on__2 1.0 0.0) :!class /Script/Engine.MaterialInstanceDynamic)
    (for _array_element (Variables|Default|GetLights)
      (Rendering|SetVisibility _array_element _on__2 false))
    (else
      (Rendering|Material|SetScalarParameterValue (Variables|Default|GetMID_IntensityEmissive) "Intensity" 0.0 :!class /Script/Engine.MaterialInstanceDynamic)
      (for _array_element_2 (Variables|Default|GetLights)
        (Rendering|SetVisibility _array_element_2 false false)))))

(fn ConstructionScript)

(fn GetPowerState
  (return false))