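; Breaker switch that toggles power on its Targets, sending its On state at BeginPlay and after switching.
; Interaction starts a looping timer that steps the mesh's roll to the open or closed angle, optionally flipped, then inverts On and updates the prompt text.
; Targets update only if MainBreaker reports power; without it, a switch that ends up off re-triggers its own interaction after a short delay.
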(event OnInteracted(NarrativeInteractable)
  (params (Interactor :type Pawn%20Object%20Reference) (InteractionComp :type Narrative%20Interaction%20Component%20Object%20Reference))
  (bind _target_rotation_open (Variables|Default|GetTarget%20Rotation_Open))
  (if (not (Variables|Default|GetOn?))
    (Variables|Default|SetTargetRotation (select (Variables|Default|GetFlip?) (* _target_rotation_open -1.0) _target_rotation_open))
    (else
      (Variables|Default|SetTargetRotation (Variables|Default|GetTarget%20Rotation_Close))))
  (bind _returnvalue (Utilities|Time|SetTimerbyFunctionName 0 "Activate" 0.001 true))
  (Variables|Default|SetActivateTimerHandle _returnvalue))

(event Custom|Activate
  (Transformation|SetRelativeRotation (Variables|Default|GetStaticMesh) (Math|Rotator|MakeRotator (Math|Interpolation|FInterptoConstant (Variables|Default|GetCurrentRotation) (Variables|Default|GetTargetRotation) (Utilities|Time|GetWorldDeltaSeconds) (Variables|Default|GetActivateSpeed)) 0.0 0.0) false false)
  (if (Variables|Default|GetOn?)
    (Variables|Default|SetCurrentRotation (+ (Variables|Default|GetCurrentRotation) (select (Variables|Default|GetFlip?) -1.0 1.0)))
    (else
      (Variables|Default|SetCurrentRotation (+ (Variables|Default|GetCurrentRotation) (select (Variables|Default|GetFlip?) 1.0 -1.0)))))
  (if (== (Variables|Default|GetCurrentRotation) (Variables|Default|GetTargetRotation))
    (Utilities|Time|ClearandInvalidateTimerbyHandle (Variables|Default|GetActivateTimerHandle))
    (Variables|Default|SetOn? (not (Variables|Default|GetOn?)))
    (Class|NarrativeInteractableComponent|SetInteractableActionText (Variables|Default|GetNarrativeInteractable) (select (Variables|Default|GetOn?) (Variables|Default|GetCloseText) (Variables|Default|GetOpenText)))
    (bind _on_ (Class|BPIElectricObject|GetPowerState(Message) (Variables|Default|GetMainBreaker)))
    (if _on_
      (Development|PrintString "Hello POWER ON")
      (CallFunction|Init)
      (else
        (Development|PrintString "Hello no POWER")
        (if (not (Variables|Default|GetOn?))
          (Utilities|FlowControl|Delay 0.1)
          (CallFunction|CEInteracted))))))

(event Custom|Init
  (for _array_element (Variables|Default|GetTargets)
    (Class|BPIElectricObject|SetPoweron(Message) _array_element (Variables|Default|GetOn?))))

(event Custom|CE_Interacted
  (bind _target_rotation_open (Variables|Default|GetTarget%20Rotation_Open))
  (if (not (Variables|Default|GetOn?))
    (Variables|Default|SetTargetRotation (select (Variables|Default|GetFlip?) (* _target_rotation_open -1.0) _target_rotation_open))
    (else
      (Variables|Default|SetTargetRotation (Variables|Default|GetTarget%20Rotation_Close))))
  (bind _returnvalue (Utilities|Time|SetTimerbyFunctionName 0 "Activate" 0.001 true))
  (Variables|Default|SetActivateTimerHandle _returnvalue))

(event EventBeginPlay
  (CallFunction|Init))

(event EventSetPoweron
  (params (On? :type Boolean))
  (Variables|Default|SetPowerOn? On?))

(fn ConstructionScript)

(fn GetPowerState
  (return (Variables|Default|GetOn?)))