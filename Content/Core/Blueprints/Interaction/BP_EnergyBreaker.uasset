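; Interactable energy breaker that toggles its enabled state when used, depending on whether the main power breaker is on.
; With main power on, a FlipFlop sets BreakerEnabled and InteractAction swaps between two stuffed-cat meshes to show the state.
; With main power off, a reset DoN runs the same toggle twice with a short delay, so the breaker flips and springs back.
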(event OnInteracted(NarrativeInteractable)
  (params (Interactor :type Pawn%20Object%20Reference) (InteractionComp :type Narrative%20Interaction%20Component%20Object%20Reference))
  (if (Variables|/Game/Core/Blueprints/Interaction/BP_MainPowerBreaker.BP_MainPowerBreaker_C|GetMainPowerOn? (Variables|Default|GetMainPowerBreaker))
    _
    (else
      (Utilities|FlowControl|Sequence
        (:then_0
          (goto _label Reset))
        (:then_1
          (Utilities|FlowControl|DoN 2 :!label _label
            (:Exit
              (Utilities|FlowControl|Sequence
                (:then_0
                  _)
                (:then_1
                  (Utilities|FlowControl|Delay 0.2)
                  (goto _label)))))))))
  (bind _isa (Utilities|FlowControl|FlipFlop)
    (:A
      (Variables|Default|SetBreakerEnabled? false))
    (:B
      (Variables|Default|SetBreakerEnabled? true)))
  (CallFunction|InteractAction _isa))

(fn ConstructionScript)

(fn InteractAction
  (params (Interacted? :type Boolean))
  (Components|StaticMesh|SetStaticMesh (Variables|Default|GetSM_Interactable) (select Interacted? "/Game/PolygonHorrorMansion/Meshes/Props/SM_Prop_Cat_Stuffed_02.SM_Prop_Cat_Stuffed_02" "/Game/PolygonHorrorMansion/Meshes/Props/SM_Prop_Cat_Stuffed_01.SM_Prop_Cat_Stuffed_01")))