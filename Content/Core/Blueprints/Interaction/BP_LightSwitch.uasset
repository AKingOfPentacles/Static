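; Interactable light switch that toggles its on/off state through a Narrative interactable, depending on whether its referenced Breaker is enabled.
; With power, interaction flips Enabled, swaps between two placeholder-looking stuffed-cat meshes and updates the action and name text.
; Without power, a DoN, FlipFlop and short delay loop briefly flicks the mesh without changing Enabled.
; BeginPlay runs the same toggle once, inverting the initial Enabled value.
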(event OnInteracted(NarrativeInteractable)
  (params (Interactor :type Pawn%20Object%20Reference) (InteractionComp :type Narrative%20Interaction%20Component%20Object%20Reference))
  (if (Variables|/Game/Core/Blueprints/Interaction/BP_EnergyBreaker.BP_EnergyBreaker_C|GetBreakerEnabled? (Variables|Default|GetBreaker))
    (if (Variables|Default|GetEnabled?)
      (Variables|Default|SetEnabled? false)
      (CallFunction|InteractAction false)
      (else
        (Variables|Default|SetEnabled? true)
        (CallFunction|InteractAction true)))
    (CallFunction|UpdateActionText)
    (CallFunction|UpdateObjectText)
    (else
      (Utilities|FlowControl|Sequence
        (:then_0
          (goto _label Reset))
        (:then_1
          (Utilities|FlowControl|DoN 2 :!label _label
            (:Exit
              (Utilities|FlowControl|Sequence
                (:then_0
                  (bind _isa (Utilities|FlowControl|FlipFlop)
                    (:A
                      _)
                    (:B
                      _))
                  (CallFunction|InteractAction _isa))
                (:then_1
                  (Utilities|FlowControl|Delay 0.2)
                  (goto _label))))))))))

(event Custom|Init
  (if (Variables|Default|GetEnabled?)
    (Variables|Default|SetEnabled? false)
    (CallFunction|InteractAction false)
    (else
      (Variables|Default|SetEnabled? true)
      (CallFunction|InteractAction true)))
  (CallFunction|UpdateActionText)
  (CallFunction|UpdateObjectText))

(event EventBeginPlay
  (CallFunction|Init)
  (CallFunction|UpdateActionText)
  (CallFunction|UpdateObjectText))

(fn ConstructionScript)

(fn InteractAction
  (params (Interacted? :type Boolean))
  (Components|StaticMesh|SetStaticMesh (Variables|Default|GetSM_Interactable) (select Interacted? "/Game/PolygonHorrorMansion/Meshes/Props/SM_Prop_Cat_Stuffed_02.SM_Prop_Cat_Stuffed_02" "/Game/PolygonHorrorMansion/Meshes/Props/SM_Prop_Cat_Stuffed_01.SM_Prop_Cat_Stuffed_01")))

(fn UpdateActionText
  (if (Variables|/Game/Core/Blueprints/Interaction/BP_EnergyBreaker.BP_EnergyBreaker_C|GetBreakerEnabled? (Variables|Default|GetBreaker))
    (Class|NarrativeInteractableComponent|SetInteractableActionText (Variables|Default|GetNarrativeInteractable) (Variables|Default|GetStatePower_Action))
    (else
      (Class|NarrativeInteractableComponent|SetInteractableActionText (Variables|Default|GetNarrativeInteractable) (Variables|Default|GetStatePower_ActionOff)))))

(fn UpdateObjectText
  (Class|NarrativeInteractableComponent|SetInteractableNameText (Variables|Default|GetNarrativeInteractable) (Utilities|Text|MakeLiteralText (select (Variables|Default|GetEnabled?) "LightOn" "LightOff"))))