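; BP_LightSwitch is an interactable wall switch that toggles linked lights, depending on a referenced power breaker.
; With breaker power, interaction flips PowerOn, updates the prompt text, animates the switch roll via a timeline, then notifies each light.
; Without power, a second timeline animates the switch without changing state.
; An Enabled flag blocks input during animation, while SetPower re-notifies the lights and GetPowerState exposes the state.
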(event OnInteracted(NarrativeInteractable)
  (params (Interactor :type Pawn%20Object%20Reference) (InteractionComp :type Narrative%20Interaction%20Component%20Object%20Reference))
  (bind _on_ (Class|BPIElectricObject|GetPowerState(Message) (Variables|Setting|GetPowerBreakerRef)))
  (if _on_
    (if (Variables|Default|GetEnabled?)
      (Variables|Default|SetEnabled? false)
      (if (Variables|Default|GetPowerOn?)
        (Variables|Default|SetPowerOn? false)
        (CallFunction|SetTextAction)
        (bind _alpha (Timeline|Timeline ReverseFromEnd)
          (:Update
            (Transformation|SetRelativeRotation (Variables|Default|GetSwitch) (Math|Rotator|MakeRotator (Math|Float|Lerp 0.0 -45.0 _alpha) 0.0 0.0) false false))
          (:Finished
            (Variables|Default|SetEnabled? true)
            (for _array_element (Variables|Setting|GetLightRef)
              (Class|BPIElectricObject|SetPower(Message) _array_element))))
        (else
          (Variables|Default|SetPowerOn? true)
          (CallFunction|SetTextAction)
          (Timeline|Timeline PlayFromStart))))
    (elif (Variables|Default|GetEnabled?)
      (Variables|Default|SetEnabled? false)
      (if (Variables|Default|GetPowerOn?)
        (bind _alpha_2 (Timeline|Timeline_0 PlayFromStart)
          (:Update
            (Transformation|SetRelativeRotation (Variables|Default|GetSwitch) (Math|Rotator|MakeRotator (Math|Float|Lerp 0.0 -45.0 _alpha_2) 0.0 0.0) false false))
          (:Finished
            (Variables|Default|SetEnabled? true)))
        (else
          (Timeline|Timeline_0 ReverseFromEnd))))))

(event EventBeginPlay
  (CallFunction|SetTextAction))

(event EventSetPower
  (for _array_element (Variables|Setting|GetLightRef)
    (Class|BPIElectricObject|SetPower(Message) _array_element)))

(fn ConstructionScript)

(fn SetTextAction
  (Class|NarrativeInteractableComponent|SetInteractableActionText (Variables|Default|GetNarrativeInteractable) (select (Variables|Default|GetPowerOn?) (Variables|Default|GetPowerOff_Text) (Variables|Default|GetPowerON_Text))))

(fn GetPowerState
  (return (Variables|Default|GetPowerOn?)))