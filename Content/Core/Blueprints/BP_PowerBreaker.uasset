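; BP_PowerBreaker is an interactable breaker that toggles a power state, exposed through GetPowerState.
; Interaction or SetPower flips PowerOn, updates the narrative interactable's action text and plays a timeline forward or backward to rotate the switch mesh.
; An Enabled flag blocks repeat interactions during animation, though SetPower bypasses it.
; When the timeline finishes, interaction re-enables and each linked switch receives SetPowerMessage.
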(event OnInteracted(NarrativeInteractable)
  (params (Interactor :type Pawn%20Object%20Reference) (InteractionComp :type Narrative%20Interaction%20Component%20Object%20Reference))
  (if (Variables|Default|GetEnabled?)
    (Variables|Default|SetEnabled? false)
    (if (Variables|Default|GetPowerOn?)
      (Variables|Default|SetPowerOn? false)
      (CallFunction|SetTextAction)
      (bind _alpha (Timeline|Timeline PlayFromStart)
        (:Update
          (Transformation|SetRelativeRotation (Variables|Default|GetPowerBox_Switch) (Math|Rotator|MakeRotator (Math|Float|Lerp 0.0 9e+01 _alpha) 0.0 0.0) false false))
        (:Finished
          (Variables|Default|SetEnabled? true)
          (for _array_element (Variables|Default|GetSwitches)
            (Class|BPIElectricObject|SetPower(Message) _array_element))))
      (else
        (Variables|Default|SetPowerOn? true)
        (CallFunction|SetTextAction)
        (Timeline|Timeline ReverseFromEnd)))))

(event EventBeginPlay
  (CallFunction|SetTextAction))

(event EventSetPower
  (if (Variables|Default|GetPowerOn?)
    (Variables|Default|SetPowerOn? false)
    (CallFunction|SetTextAction)
    (bind _alpha (Timeline|Timeline PlayFromStart)
      (:Update
        (Transformation|SetRelativeRotation (Variables|Default|GetPowerBox_Switch) (Math|Rotator|MakeRotator (Math|Float|Lerp 0.0 9e+01 _alpha) 0.0 0.0) false false))
      (:Finished
        (Variables|Default|SetEnabled? true)
        (for _array_element (Variables|Default|GetSwitches)
          (Class|BPIElectricObject|SetPower(Message) _array_element))))
    (else
      (Variables|Default|SetPowerOn? true)
      (CallFunction|SetTextAction)
      (Timeline|Timeline ReverseFromEnd))))

(fn ConstructionScript)

(fn SetTextAction
  (Class|NarrativeInteractableComponent|SetInteractableActionText (Variables|Default|GetNarrativeInteractable) (select (Variables|Default|GetPowerOn?) (Variables|Default|GetPowerOff_Text) (Variables|Default|GetPowerON_Text))))

(fn GetPowerState
  (return (Variables|Default|GetPowerOn?)))