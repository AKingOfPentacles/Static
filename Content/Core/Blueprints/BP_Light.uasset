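; BP_Light is a light actor whose point light depends on the power state of a power box and a switch.
; SetPower queries both through GetPowerState interface messages, showing the light only when both report power and hiding it otherwise.
; Its own GetPowerState always returns false, and it runs no logic on Tick or BeginPlay.
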(event EventBeginPlay)

(event Collision|EventActorBeginOverlap
  (params (OtherActor :type Actor%20Object%20Reference)))

(event EventTick
  (params (DeltaSeconds :type Float%20%28single-precision%29)))

(event EventSetPower
  (bind _on_ (Class|BPIElectricObject|GetPowerState(Message) (Variables|Default|GetPowerBox)))
  (if _on_
    (bind _on__2 (Class|BPIElectricObject|GetPowerState(Message) (Variables|Default|GetSwitch)))
    (Rendering|SetVisibility (Variables|Default|GetPointLight) _on__2 false)
    (else
      (Rendering|SetVisibility (Variables|Default|GetPointLight) false false))))

(fn ConstructionScript)

(fn GetPowerState
  (return false))