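; BP_Clock is an analog clock actor that runs at roughly 128 times real speed and triggers a power event.
; A fast looping timer started on BeginPlay rotates the hour, minute and second hand meshes, then advances the time counters by one second per call.
; Once Minutes reaches 15, a DoOnce calls SetPowerMessage on the PowerBox.
; Each timer call also prints the current minutes.
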(event Custom|ClockTimer
  (Development|PrintString (Utilities|String|ToString(Integer) (Variables|Default|GetMinutes)))
  (Transformation|SetRelativeRotation (Variables|Default|GetSM_Prop_Clock_01_Hand_Hour) (Math|Rotator|MakeRotator 0.0 (* (+ (Math|Conversions|ToFloat(Integer) (* (Variables|Default|GetHours) 30)) (/ (Variables|Default|GetMinutes) 2)) -1.0) 0.0) false false)
  (Transformation|SetRelativeRotation (Variables|Default|GetSM_Prop_Clock_01_Hand_Minutes) (Math|Rotator|MakeRotator 0.0 (+ (* (Variables|Default|GetMinutes) -6) -9e+01) 0.0) false false)
  (Transformation|SetRelativeRotation (Variables|Default|GetSM_Prop_Clock_01_Hand_Seconds) (Math|Rotator|MakeRotator 0.0 (+ (* (Variables|Default|GetSeconds) -6) -90) 0.0) false false)
  (Utilities|FlowControl|Sequence
    (:then_0
      (if (>= (Variables|Default|GetMinutes) 15)
        (Utilities|FlowControl|DoOnce false
          (:Completed
            (Class|BPIElectricObject|SetPower(Message) (Variables|Default|GetPowerBox))))))
    (:then_1
      (Math|Integer|IncrementInt (Variables|Default|GetSeconds)
        (:%20%20
          (if (== (Variables|Default|GetSeconds) 60)
            (Variables|Default|SetSeconds 0)
            (Math|Integer|IncrementInt (Variables|Default|GetMinutes)
              (:%20%20
                (if (== (Variables|Default|GetMinutes) 60)
                  (Variables|Default|SetMinutes 0)
                  (Math|Integer|IncrementInt (Variables|Default|GetHours)))))))))))

(event EventBeginPlay
  (Utilities|Time|SetTimerbyFunctionName 0 "ClockTimer" 0.007812 true))

(fn ConstructionScript)