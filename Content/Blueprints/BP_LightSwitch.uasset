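; Light switch actor that toggles its PowerOn state on interaction through a NarrativeInteractable and has its linked Lights re-check their power.
; On BeginPlay it binds to the referenced power breaker's PowerBreakerCheck dispatcher and to its own ElectricObjectCheck.
; Breaker changes and interactions both broadcast ElectricObjectCheck, whose handler calls CheckPower on each light.
; TogglePower and ToggleOn only call their parent versions, and debug prints remain in both check handlers.
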(event OnInteracted(NarrativeInteractable)
  (params (Interactor :type Pawn%20Object%20Reference) (InteractionComp :type Narrative%20Interaction%20Component%20Object%20Reference))
  (Variables|Default|SetPowerOn? (not (Variables|Default|GetPowerOn?)))
  (Default|CallElectricObjectCheck))

(event Custom|PowerBreakerCheck_Event_0
  (Development|PrintString "Hello Power Breaker")
  (Default|CallElectricObjectCheck))

(event Custom|ElectricObjectCheck_Event
  (Development|PrintString "Hello Electric Objects")
  (for _array_element (Variables|Default|GetLights)
    (Default|CheckPower _array_element)))

(event EventBeginPlay
  (EventDispatchers|AssignPowerBreakerCheck (Variables|Default|GetPowerBreakerRef) (delegate Custom|PowerBreakerCheck_Event_0))
  (EventDispatchers|AssignElectricObjectCheck (delegate Custom|ElectricObjectCheck_Event)))

(event Collision|EventActorBeginOverlap
  (params (OtherActor :type Actor%20Object%20Reference)))

(event EventTick
  (params (DeltaSeconds :type Float%20%28single-precision%29)))

(fn ConstructionScript)

(fn TogglePower
  (|CallParentFunction))

(fn Toggleon
  (|CallParentFunction))