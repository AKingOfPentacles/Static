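; Neon light controller Blueprint that switches arrays of referenced point, spot and rect lights on or off.
; The construction script and BeginPlay set the initial state from the IsOn flag, so it also previews in the editor.
; CheckPower lights them only when both the referenced switch and that switch's power breaker are on.
; ActivateLights and DeActivateLights toggle each light component's visibility.
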(event Custom|CheckPower
  (bind _switchref (Variables|Default|GetSwitchRef))
  (if (and (Variables|/Game/Blueprints/BP_ElectricObject.BP_ElectricObject_C|GetPowerOn? _switchref) (Variables|/Game/Blueprints/BP_PowerBreakerr.BP_PowerBreakerr_C|GetPowerBreakerOn? (Variables|/Game/Blueprints/BP_ElectricObject.BP_ElectricObject_C|GetPowerBreakerRef _switchref)))
    (CallFunction|ActivateLights)
    (else
      (CallFunction|DeActivateLights))))

(event EventBeginPlay
  (if (Variables|Default|GetisOn?)
    (CallFunction|ActivateLights)
    (else
      (CallFunction|DeActivateLights))))

(fn ConstructionScript
  (if (Variables|Default|GetisOn?)
    (CallFunction|ActivateLights)
    (else
      (CallFunction|DeActivateLights))))

(fn ActivateLights
  (Utilities|FlowControl|Sequence
    (:then_0
      (if (Utilities|Array|IsValidIndex (Variables|Default|GetPointLights))
        (for _array_element (Variables|Default|GetPointLights)
          (Rendering|SetVisibility (Variables|/Script/Engine.Light|GetLightComponent _array_element) true false))))
    (:then_1
      (if (Utilities|Array|IsValidIndex (Variables|Default|GetSpotLights))
        (for _array_element_2 (Variables|Default|GetSpotLights)
          (Rendering|SetVisibility (Variables|/Script/Engine.Light|GetLightComponent _array_element_2) true false))))
    (:then_2
      (if (Utilities|Array|IsValidIndex (Variables|Default|GetRectLights))
        (for _array_element_3 (Variables|Default|GetRectLights)
          (Rendering|SetVisibility (Variables|/Script/Engine.Light|GetLightComponent _array_element_3) true false))))))

(fn DeActivateLights
  (Utilities|FlowControl|Sequence
    (:then_0
      (if (Utilities|Array|IsValidIndex (Variables|Default|GetPointLights))
        (for _array_element (Variables|Default|GetPointLights)
          (Rendering|SetVisibility (Variables|/Script/Engine.Light|GetLightComponent _array_element) false false))))
    (:then_1
      (if (Utilities|Array|IsValidIndex (Variables|Default|GetSpotLights))
        (for _array_element_2 (Variables|Default|GetSpotLights)
          (Rendering|SetVisibility (Variables|/Script/Engine.Light|GetLightComponent _array_element_2) false false))))
    (:then_2
      (if (Utilities|Array|IsValidIndex (Variables|Default|GetRectLights))
        (for _array_element_3 (Variables|Default|GetRectLights)
          (Rendering|SetVisibility (Variables|/Script/Engine.Light|GetLightComponent _array_element_3) false false))))))