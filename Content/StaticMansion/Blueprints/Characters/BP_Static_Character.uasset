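; Player character built on ALS that shows a held prop and animation style for the current overlay mode.
; Overlay changes link the matching animation layer and swap static or skeletal meshes on hand sockets or gun bones.
; Non-low mantles and ragdolling hide the prop until they end, and low mantle settings vary by overlay.
; A debug E key prints the game phase's remaining time.
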(event EventOnOverlayModeChanged
  (params (PreviousOverlayMode :type Gameplay%20Tag%20Structure%20%28by%20ref%29))
  (Overlay|RefreshOverlayLinkedAnimationLayer)
  (Overlay|RefreshOverlayObject))

(event EventOnMantlingEnded
  (Overlay|RefreshOverlayObject))

(event EventOnRagdollingEnded
  (Overlay|RefreshOverlayObject))

(event EventOnMantlingStarted
  (params (Parameters :type Als%20Mantling%20Parameters%20Structure%20%28by%20ref%29))
  (if (Utilities|Enum|NotEqual(Enum) (.mantlingtype Parameters) "Low")
    (Overlay|ClearOverlayObject)))

(event EventBeginPlay
  (Overlay|RefreshOverlayObject))

(event EventOnRagdollingStarted
  (Overlay|ClearOverlayObject))

(event Input|KeyboardEvents|DebugKeyE
  (params (Key :type Key%20Structure) (ActionValue :type Input%20Action%20Value%20Structure))
  (:Pressed
    (Development|PrintString (Utilities|String|ToString(Float) (Class|GamePhaseManager|GetPhaseTimeRemaining (Subsystems|GetGamePhaseManager))))))

(fn ConstructionScript)

(fn RefreshOverlayLinkedAnimationLayer
  (bind _mesh (Variables|Character|GetMesh))
  (LocalVariables|SetOverlayAnimationInstanceClass (.Value (Utilities|Map|Find (Variables|Settings|AlsCharacter|GetOverlayAnimationInstanceClasses) (Variables|Default|GetOverlayMode))))
  (bind _overlayanimationinstanceclass (LocalVariables|GetOverlayAnimationInstanceClass)
    (:then
      (Components|SkeletalMesh|AnimationBlueprintLinking|LinkAnimClassLayers _mesh _overlayanimationinstanceclass))
    (:else
      (Components|SkeletalMesh|AnimationBlueprintLinking|LinkAnimClassLayers _mesh "/ALS/ALS/Character/AnimationInstances/Overlays/AB_Als_Default.AB_Als_Default_C"))))

(fn RefreshOverlayObject
  (|SwitchGameplayTag (Variables|Default|GetOverlayMode)
    (:Default
      (Overlay|ClearOverlayObject))
    (:Als.OverlayMode.M4
      (Overlay|AttachOverlayObject 0 "/ALS/ALS/OverlayObjects/M4/SKM_Als_M4.SKM_Als_M4" 0 "M4" false))
    (:Als.OverlayMode.PistolOneHanded
      (Overlay|AttachOverlayObject 0 "/ALS/ALS/OverlayObjects/M9/SKM_Als_M9.SKM_Als_M9" 0 "M9" false :!label _label))
    (:Als.OverlayMode.PistolTwoHanded
      (goto _label))
    (:Als.OverlayMode.Bow
      (Overlay|AttachOverlayObject 0 "/ALS/ALS/OverlayObjects/Bow/SKM_Als_Bow.SKM_Als_Bow" "/ALS/ALS/OverlayObjects/Bow/AB_Als_Bow.AB_Als_Bow_C" "Bow" true))
    (:Als.OverlayMode.Torch
      (Overlay|AttachOverlayObject "/ALS/ALS/OverlayObjects/Torch/SM_Als_Torch.SM_Als_Torch" 0 0 "Torch" true))
    (:Als.OverlayMode.Binoculars
      (Overlay|AttachOverlayObject "/ALS/ALS/OverlayObjects/Binoculars/SM_Als_Binoculars.SM_Als_Binoculars" 0 0 "Binoculars" false))
    (:Als.OverlayMode.Box
      (Overlay|AttachOverlayObject "/ALS/ALS/OverlayObjects/Box/SM_Als_Box.SM_Als_Box" 0 0 "Box" false))
    (:Als.OverlayMode.Barrel
      (Overlay|AttachOverlayObject "/ALS/ALS/OverlayObjects/Barrel/SM_Als_Barrel.SM_Als_Barrel" 0 0 "Barrel" true))))

(fn AttachOverlayObject
  (params (NewStaticMesh :type Static%20Mesh%20Object%20Reference) (NewSkeletalMesh :type Skeletal%20Mesh%20Object%20Reference) (NewAnimationClass :type Anim%20Instance%20Class%20Reference) (SocketName :type Name) (bUseLeftGunBone :type Boolean))
  (LocalVariables|SetResultSocketName (select (Variables|Settings|AlsCharacter|GetbUseGunBoneForOverlayObjects) (select bUseLeftGunBone (Class|AlsConstants|HandLeftGunVirtualBoneName) (Class|AlsConstants|HandRightGunVirtualBoneName)) SocketName))
  (Utilities|FlowControl|Sequence
    (:then_0
      (Components|StaticMesh|SetStaticMesh (Variables|Default|GetOverlayStaticMesh) NewStaticMesh)
      (Transformation|AttachComponentToComponent (Variables|Default|GetOverlayStaticMesh) (Variables|Character|GetMesh) (LocalVariables|GetResultSocketName) "SnapToTarget" "SnapToTarget" "SnapToTarget" true))
    (:then_1
      (Components|SkinnedMesh|SetSkinnedAssetandUpdate (Variables|Default|GetOverlaySkeletalMesh) NewSkeletalMesh true)
      (Class|SkeletalMeshComponent|SetAnimClass (Variables|Default|GetOverlaySkeletalMesh) NewAnimationClass)
      (Transformation|AttachComponentToComponent (Variables|Default|GetOverlaySkeletalMesh) (Variables|Character|GetMesh) (LocalVariables|GetResultSocketName) "SnapToTarget" "SnapToTarget" "SnapToTarget" true))))

(fn ClearOverlayObject
  (Components|StaticMesh|SetStaticMesh (Variables|Default|GetOverlayStaticMesh) 0)
  (Components|SkinnedMesh|SetSkinnedAssetandUpdate (Variables|Default|GetOverlaySkeletalMesh) 0 true)
  (Class|SkeletalMeshComponent|SetAnimClass (Variables|Default|GetOverlaySkeletalMesh)))

(fn SelectMantlingSettings
  (params (MantlingType :type EAlsMantlingType%20Enum :default "High"))
  (switch Utilities|FlowControl|Switch|SwitchonEAlsMantlingType MantlingType
    (:High
      _)
    (:Low
      (|SwitchGameplayTag (Variables|Default|GetOverlayMode)
        (:Default
          (return "/ALS/ALS/Data/Character/Mantle/MS_Als_Low.MS_Als_Low"))
        (:Als.OverlayMode.Injured
          _)
        (:Als.OverlayMode.HandsTied
          (return "/ALS/ALS/Data/Character/Mantle/MS_Als_Low_BothHands.MS_Als_Low_BothHands"))
        (:Als.OverlayMode.M4
          (return "/ALS/ALS/Data/Character/Mantle/MS_Als_Low_Right.MS_Als_Low_Right"))
        (:Als.OverlayMode.PistolOneHanded
          (return "/ALS/ALS/Data/Character/Mantle/MS_Als_Low_Right.MS_Als_Low_Right"))
        (:Als.OverlayMode.PistolTwoHanded
          (return "/ALS/ALS/Data/Character/Mantle/MS_Als_Low_Right.MS_Als_Low_Right"))
        (:Als.OverlayMode.Bow
          _)
        (:Als.OverlayMode.Torch
          _)
        (:Als.OverlayMode.Binoculars
          (return "/ALS/ALS/Data/Character/Mantle/MS_Als_Low_Right.MS_Als_Low_Right"))
        (:Als.OverlayMode.Box
          (return "/ALS/ALS/Data/Character/Mantle/MS_Als_Low_Box.MS_Als_Low_Box"))
        (:Als.OverlayMode.Barrel
          _))
      (return "/ALS/ALS/Data/Character/Mantle/MS_Als_Low_Left.MS_Als_Low_Left"))
    (:InAir
      _))
  (return "/ALS/ALS/Data/Character/Mantle/MS_Als_High.MS_Als_High"))